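; Spider enemy that senses PunchBag actors and damages them with capsule colliders on four legs.
; Pawn sensing writes the seen PunchBag to the blackboard for the AI behavior tree.
; AttackTarget and StopAttack set the IsAttacking animation flag and toggle leg collision.
; Leg overlaps share one ApplyDamage call using the LeftLeg1 cast result, with collision live throughout the attack rather than timed by anim notifies.
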(event `self.LeftLeg1.OnComponentBeginOverlap`
  (params (OverlappedComponent :type "PrimitiveComponent Object Reference") (OtherActor :type "Actor Object Reference") (OtherComp :type "PrimitiveComponent Object Reference") (OtherBodyIndex :type Integer) (bFromSweep :type Boolean) (SweepResult :type "HitResult Structure (by ref)"))
  ;[1 1 1] Appl,y damage to Object
  (bind _aspunch_bag (cast `/Game/Enemys/PunchBag` OtherActor)
    (:`then`
      (`GameplayStatics.ApplyDamage` _aspunch_bag (`self.AttackOneDamage`) :!label _label))
    (:`CastFailed`
      (`KismetSystemLibrary.PrintString` "I failed" true true (struct :`R` 1.0 :`G` 0.143594 :`A` 1.0) :!label _label_2))))

(event `AttackTarget`
  ;[1 1 1] Event triggered from Attack Task in AI behaviour tree to drive animation blueprint
  (set `self.IsAttacking` true)
  ;[1 1 1] Set Collsion for spider legs capsules for attack to cause overlap and give damage when attacking. Note its probably better to use animation notifies to control exactly when to make the capsules cause damage other wise player could walk into leg and get damage for example
  (`PrimitiveComponent.SetCollisionEnabled` (`self.LeftLeg2`) "QueryAndPhysics")
  (`PrimitiveComponent.SetCollisionEnabled` (`self.RightLeg1`) "QueryAndPhysics")
  (`PrimitiveComponent.SetCollisionEnabled` (`self.RightLeg2`) "QueryAndPhysics")
  (`PrimitiveComponent.SetCollisionEnabled` (`self.LeftLeg1`) "QueryAndPhysics"))

(event `self.LeftLeg2.OnComponentBeginOverlap`
  (params (OverlappedComponent :type "PrimitiveComponent Object Reference") (OtherActor :type "Actor Object Reference") (OtherComp :type "PrimitiveComponent Object Reference") (OtherBodyIndex :type Integer) (bFromSweep :type Boolean) (SweepResult :type "HitResult Structure (by ref)"))
  ;[1 1 1] Appl,y damage to Object
  (cast `/Game/Enemys/PunchBag` OtherActor
    (:`then`
      (goto _label))
    (:`CastFailed`
      (goto _label_2))))

(event `StopAttack`
  ;[1 1 1] Event triggered from Attack Task in AI behaviour tree to drive animation blueprint
  (set `self.IsAttacking` false)
  ;[1 1 1] Set Collsion for spider legs capsules for attack to cause overlap and give damage when attacking. Note its probably better to use animation notifies to control exactly when to make the capsules cause damage other wise player could walk into leg and get damage for example
  (`PrimitiveComponent.SetCollisionEnabled` (`self.RightLeg1`) "NoCollision")
  (`PrimitiveComponent.SetCollisionEnabled` (`self.LeftLeg2`) "NoCollision")
  (`PrimitiveComponent.SetCollisionEnabled` (`self.RightLeg2`) "NoCollision")
  (`PrimitiveComponent.SetCollisionEnabled` (`self.LeftLeg1`) "NoCollision"))

(event `self.RightLeg1.OnComponentBeginOverlap`
  (params (OverlappedComponent :type "PrimitiveComponent Object Reference") (OtherActor :type "Actor Object Reference") (OtherComp :type "PrimitiveComponent Object Reference") (OtherBodyIndex :type Integer) (bFromSweep :type Boolean) (SweepResult :type "HitResult Structure (by ref)"))
  ;[1 1 1] Appl,y damage to Object
  (cast `/Game/Enemys/PunchBag` OtherActor
    (:`then`
      (goto _label))
    (:`CastFailed`
      (goto _label_2))))

(event `self.PawnSensing.OnSeePawn`
  (params (Pawn :type "Pawn Object Reference"))
  ;[1 1 1] On sensing target set blackboard values to drive AI controllers behaviour tree
  (bind _aspunch_bag (cast `/Game/Enemys/PunchBag` Pawn))
  (`BlackboardComponent.SetValueAsObject` (`AIBlueprintHelperLibrary.GetBlackboard` self) "PunchBag" _aspunch_bag))

(event `self.RightLeg2.OnComponentBeginOverlap`
  (params (OverlappedComponent :type "PrimitiveComponent Object Reference") (OtherActor :type "Actor Object Reference") (OtherComp :type "PrimitiveComponent Object Reference") (OtherBodyIndex :type Integer) (bFromSweep :type Boolean) (SweepResult :type "HitResult Structure (by ref)"))
  ;[1 1 1] Appl,y damage to Object
  (cast `/Game/Enemys/PunchBag` OtherActor
    (:`then`
      (goto _label))
    (:`CastFailed`
      (goto _label_2))))

(fn `UserConstructionScript`)